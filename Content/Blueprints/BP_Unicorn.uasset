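; Unicorn actor that hops along a list of node positions, fleeing onward whenever the side-scroller player gets close.
; At each stop it spawns a BP_Fart once, then waits until a sphere overlap check on Tick detects the player.
; It then turns its mesh and makes a swept SetActorLocation jump to the next node, using the return value as arrival.
; It destroys itself after the last node.
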(event Custom|Fart
  (Game|SpawnActorfromClass "/Game/Blueprints/BP_Fart.BP_Fart_C" (Transformation|GetWorldTransform (Variables|Default|GetStaticMesh)) "Undefined" 0 0))

(event EventTick
  (params (DeltaSeconds :type Float%20%28single-precision%29))
  (bind _self self)
  (bind _staticmesh (Variables|Default|GetStaticMesh _self))
  (Utilities|FlowControl|Sequence
    (:then_0
      (if (Variables|Default|GetAtTarget)
        (if (Variables|Default|GetFarted)
          _
          (else
            (CallFunction|Fart)
            (Variables|Default|SetFarted true)))
        (if (Variables|Default|GetIsPlayerInRange)
          (Transformation|SetWorldRotation _staticmesh "0,180.000000, 0" false false)
          (bind _output_get (Variables|Default|SetIndex (+ (Variables|Default|GetIndex) 1)))
          (if (< _output_get (Utilities|Array|Length (Variables|Default|GetNodes)))
            (Variables|Default|SetTarget (Utilities|Array|Get(acopy) (Variables|Default|GetNodes) (Variables|Default|GetIndex)))
            (Variables|Default|SetAtTarget false)
            (Variables|Default|SetFarted false)
            (else
              (Actor|DestroyActor)))
          (else
            (Transformation|SetWorldRotation _staticmesh "0, 0, 0" false false)))
        (else
          (bind _returnvalue (Transformation|SetActorLocation (Variables|Default|GetTarget) true false))
          (Variables|Default|SetAtTarget _returnvalue))))
    (:then_1
      (Variables|Default|SetIsPlayerInRange (> (Utilities|Array|Length (Collision|GetOverlappingActors (Variables|Default|GetSphere) "/Game/Blueprints/SideScrollerCharacter.SideScrollerCharacter_C" :!class /Script/Engine.PrimitiveComponent)) 0)))))

(event EventBeginPlay
  (Variables|Default|SetTarget (Utilities|Array|Get(acopy) (Variables|Default|GetNodes) (Variables|Default|GetIndex))))

(fn ConstructionScript)