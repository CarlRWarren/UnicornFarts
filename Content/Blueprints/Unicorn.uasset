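; Unicorn actor that hops along negative Y at X zero and random heights, farting after successful moves.
; Tick alternates between a swept SetActorLocation straight to Target, whose return value sets AtTarget, and choosing the next random Target.
; Before each new Target is picked, Fart spawns an actor (class not shown) at the mesh's world transform.
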(event Custom|Fart
  (Game|SpawnActorfromClass "/Game/Blueprints/BP_Fart.BP_Fart_C" (Transformation|GetWorldTransform (Variables|Character|GetMesh)) "Undefined" 0 0))

(event EventTick
  (params (DeltaSeconds :type Float%20%28single-precision%29))
  (if (Variables|Default|GetAtTarget)
    (CallFunction|Fart)
    (Variables|Default|SetTarget (Math|Vector|MakeVector 0.0 (- (.y (Transformation|GetActorLocation)) (Math|Random|RandomFloatinRange 5e+01 1.5e+02)) (Math|Random|RandomFloatinRange 1.3e+02 4e+02)))
    (Variables|Default|SetAtTarget false)
    (else
      (bind _returnvalue (Transformation|SetActorLocation (Variables|Default|GetTarget) true false))
      (Variables|Default|SetAtTarget _returnvalue))))

(fn ConstructionScript)